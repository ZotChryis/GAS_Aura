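; BP_EnemyBase is the Blueprint base for enemies, handling spawn, facing and dissolve presentation.
; On BeginPlay a timeline scales the mesh through its Spawn curve.
; UpdateFacingTarget sets the FacingTarget warp location on the Motion Warping component.
; Two further events run timelines that drive the Dissolve scalar parameter on passed-in dynamic materials, separately for body and weapon.
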(event `self.ReceiveBeginPlay`
  (bind (_direction _scale) (`Timeline|Spawn`)
    (:`Update`
      (`SceneComponent.SetRelativeScale3D` (`self.Mesh`) (`KismetMathLibrary.MakeVector` _scale _scale _scale)))))

(event `CombatInterface.UpdateFacingTarget`
  (params (TargetFacing :type "Vector Structure (by ref)"))
  (`MotionWarpingComponent.AddOrUpdateWarpTargetFromLocation` (`self.MotionWarping`) "FacingTarget" TargetFacing))

(event `self.StartDissolveTimeline`
  (params (DynamicMaterialInstance :type "MaterialInstanceDynamic Object Reference"))
  (bind (_direction _dissolvetrack) (`Timeline|Dissolve`)
    (:`Update`
      (`MaterialInstanceDynamic.SetScalarParameterValue` DynamicMaterialInstance "Dissolve" _dissolvetrack))))

(event `self.StartWeaponDissolveTimeline`
  (params (DynamicMaterialInstance :type "MaterialInstanceDynamic Object Reference"))
  (bind (_direction _weapon_dissolve) (`Timeline|Weapon Dissolve`)
    (:`Update`
      (`MaterialInstanceDynamic.SetScalarParameterValue` DynamicMaterialInstance "Dissolve" _weapon_dissolve))))

(fn `UserConstructionScript`)