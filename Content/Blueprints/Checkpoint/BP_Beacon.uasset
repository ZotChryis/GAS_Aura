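; BP_Beacon is a checkpoint beacon that lights up and marks itself reached when the player touches it.
; Overlapping its sphere with an actor implementing PlayerInterface calls HandleGlowEffects and sets the Reached flag.
; The CheckpointReached event receives a dynamic material instance and plays a timeline that drives its Glow parameter, scaled by GlowFactor.
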(event `self.Sphere.OnComponentBeginOverlap`
  (params (OverlappedComponent :type "PrimitiveComponent Object Reference") (OtherActor :type "Actor Object Reference") (OtherComp :type "PrimitiveComponent Object Reference") (OtherBodyIndex :type Integer) (bFromSweep :type Boolean) (SweepResult :type "HitResult Structure (by ref)"))
  (if (`KismetSystemLibrary.DoesImplementInterface` OtherActor "/Script/Aura.PlayerInterface")
    (`self.HandleGlowEffects`)
    (set `self.bReached` true)))

(event `self.CheckpointReached`
  (params (DynamicMaterialInstance :type "MaterialInstanceDynamic Object Reference"))
  (bind (_direction _beacontrack) (`Timeline|BeaconTimeline` :!via `PlayFromStart`)
    (:`Update`
      (`MaterialInstanceDynamic.SetScalarParameterValue` DynamicMaterialInstance "Glow" (* _beacontrack (`self.GlowFactor`))))))

(fn `UserConstructionScript`
  (`parent.UserConstructionScript`))