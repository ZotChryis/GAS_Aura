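; Gameplay ability for the goblin spearman's melee attack, currently drawing debug spheres in place of applying damage.
; It turns the avatar toward its combat target through CombatInterface and plays the spear attack montage, ending when the montage completes, is interrupted or is cancelled.
; On the melee montage gameplay event, it finds live players within a small radius of the combat socket and marks the socket and each player found.
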(event `self.K2_ActivateAbility`
  (bind _returnvalue (`self.GetAvatarActorFromActorInfo`))
  (bind _ascombat_interface (cast `CombatInterface` _returnvalue)
    (:`then`
      (set `self.CombatInterface` _ascombat_interface)
      (bind _returnvalue_2 (message `EnemyInterface.GetCombatTarget` _returnvalue))
      (`CombatInterface.UpdateFacingTarget` _ascombat_interface (`Actor.K2_GetActorLocation` _returnvalue_2))
      (`AbilityTask_PlayMontageAndWait.CreatePlayMontageAndWaitProxy` "None" "/Game/Assets/Enemies/Goblin/Animations/Spear/AM_Attack_Spear.AM_Attack_Spear"
        (:`then`
          (`AbilityTask_WaitGameplayEvent.WaitGameplayEvent` (struct :`TagName` "Event.Montage.Melee") null
            (:`EventReceived`
              (bind _returnvalue_3 (`CombatInterface.GetCombatSocketLocation` (`self.CombatInterface`)))
              (`KismetSystemLibrary.DrawDebugSphere` _returnvalue_3 50.0 12 (struct :`R` 1.0 :`G` 0.062269 :`B` 0.082164 :`A` 1.0) 0.75)
              (bind _outactors (`AuraAbilitySystemLibrary.GetLivePlayersWithinRadius` _returnvalue (`|MakeArray` _returnvalue) _returnvalue_3 50.0))
              (for _array_element _outactors
                (`KismetSystemLibrary.DrawDebugSphere` (`Actor.K2_GetActorLocation` _array_element) 15.0 12 (struct :`R` 0.329924 :`G` 0.86979 :`B` 1.0 :`A` 1.0) 0.75)))))
        (:`OnCompleted`
          (`self.K2_EndAbility` :!label _label))
        (:`OnInterrupted`
          (goto _label))
        (:`OnCancelled`
          (goto _label))))
    (:`CastFailed`
      (`self.K2_EndAbility`))))