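; Electrocute is a channeled Gameplay Ability that fires a lightning beam at the target under the mouse, chaining to additional targets.
; A montage event spawns looping shock cues and starts a timer that pays cost and applies damage until input release, failed cost or primary target death.
; Additional targets' cues are tracked in a map and removed on death.
; Ending restores movement and cleans up, applying cooldown and final debuff damage if cast.
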(event `self.K2_ActivateAbility`
  (if (`KismetSystemLibrary.DoesImplementInterface` (`self.GetAvatarActorFromActorInfo`) "/Script/Aura.CombatInterface")
    ; Initial Data Setup for Mouse
    (bind (_asynctaskproxy _datahandle) (`TargetDataUnderMouse.CreateTargetDataUnderMouse`)
      (:`Data`
        (`self.StoreMouseDataInfo` (`AbilitySystemBlueprintLibrary.GetHitResultFromTargetData` _datahandle))
        (`self.StoreOwnerVariables`)
        (`|ExecutionSequence`
          (:`then_0`
            ; Mouse, Movement, & Animation
            (set `PlayerController.bShowMouseCursor` false (`self.OwnerPlayerController`))
            (message `CombatInterface.UpdateFacingTarget` (`self.GetAvatarActorFromActorInfo`) (`self.MouseHitLocation`))
            (`self.K2_ExecuteGameplayCue` (struct :`TagName` "GameplayCue.Shock.Cast"))
            (`AbilityTask_PlayMontageAndWait.CreatePlayMontageAndWaitProxy` "None" "/Game/Assets/Characters/Aura/Animations/Abilities/AM_Cast_Shock.AM_Cast_Shock" 1.0 "None" false
              (:`then`
                (`AbilityTask_WaitGameplayEvent.WaitGameplayEvent` (struct :`TagName` "Event.Montage.Electrocute") null
                  (:`EventReceived`
                    (message `CombatInterface.SetInCastLoop` (`self.GetAvatarActorFromActorInfo`) true)
                    (`CharacterMovementComponent.DisableMovement` (`Character.CharacterMovement` (`self.OwnerCharacter`)))
                    (set `self.ShouldApplyCooldown` true)
                    (`self.SpawnBeam`)
                    ; Tick Damage and Cost - Ends if can't pay cost
                    (bind _returnvalue (`KismetSystemLibrary.K2_SetTimerDelegate` (delegate `DamageAndCost`) (`self.DamageDeltaTime`) true))
                    (set `self.DamageAndCostTimer` _returnvalue))))))
          (:`then_1`
            ; Wait for Mouse Release to End Ability
            (`AbilityTask_WaitInputRelease.WaitInputRelease` false
              (:`OnRelease`
                (`self.K2_EndAbility`)))))))
    (else
      (`self.K2_EndAbility`))))

(event `DamageAndCost`
  ; Tick Damage and Cost - Ends if can't pay cost
  (if (`self.IsFirstTargetDead`)
    (`self.K2_EndAbility` :!label _label)
    (else
      (bind _returnvalue (`self.K2_CommitAbilityCost` false))
      (if _returnvalue
        (`self.ApplyDamage`)
        (else
          (goto _label))))))

(event `self.K2_OnEndAbility`
  (params (bWasCancelled :type Boolean))
  ; Mouse, Movement, & Animation Ending
  (set `PlayerController.bShowMouseCursor` true (`self.OwnerPlayerController`))
  (message `CombatInterface.SetInCastLoop` (`self.GetAvatarActorFromActorInfo`) false)
  (`CharacterMovementComponent.SetMovementMode` (`Character.CharacterMovement` (`self.OwnerCharacter`)) "MOVE_Walking" 0)
  ; Cleanup Cues and Timer
  (`self.RemoveCuesAndShock`)
  (`KismetSystemLibrary.K2_ClearAndInvalidateTimerHandle` (`self.DamageAndCostTimer`))
  ; Apply Cooldown if we actually casted
  (if (`self.ShouldApplyCooldown`)
    (set `self.ShouldApplyCooldown` false)
    (`self.K2_CommitAbilityCooldown` false)
    ; Issue Final 'Damage'  for Debuff Effects
    (`/Engine/EditorBlueprintResources/StandardMacros.IsValid` (`self.MouseHitActor`)
      (:`Is Valid`
        (if (`self.FirstTargetImplementsInterface`)
          (bind _ascombat_interface (cast `CombatInterface` (`self.MouseHitActor`)))
          (if (not (`CombatInterface.IsDead` _ascombat_interface))
            (`AuraAbilitySystemLibrary.ApplyDamageEffect` (`self.MakeDamageEffectParamsFromClassDefaults` (`self.MouseHitActor`)))))))))

(event `self.PrimaryTargetDied`
  (params (DeadActor :type "Actor Object Reference"))
  (`self.K2_EndAbility`))

(event `self.AdditionalTargetDied`
  (params (DeadActor :type "Actor Object Reference"))
  (`self.RemoveCueFromAddtionalTarget` DeadActor))

(fn `AddCueToAdditionalTarget`
  (params (Actor :type "Actor Object Reference"))
  (locals (Target :type "Actor Object Reference"))
  (bind _returnvalue (`AbilitySystemBlueprintLibrary.MakeGameplayCueParameters` 0.0 0.0 (struct) (struct) (struct) (struct) (struct) (`Actor.K2_GetActorLocation` (`local.Target`)) (0.0 0.0 0.0) null null (`local.Target`) null 1 1 (`Actor.RootComponent` (`self.MouseHitActor`))))
  (bind _output_get (set `local.Target` Actor))
  (`BlueprintMapLibrary.Map_Add` (`self.AdditionalTargetsToCueParams`) _output_get _returnvalue)
  (`GameplayCueFunctionLibrary.AddGameplayCueOnActor` (`local.Target`) (struct :`TagName` "GameplayCue.Shock.Loop") _returnvalue))

(fn `ApplyDamage`
  (locals (ASC :type "AbilitySystemComponent Object Reference") (EffectContext :type "GameplayEffectSpecHandle Structure"))
  (bind _returnvalue (`self.GetAbilitySystemComponentFromActorInfo`))
  (bind _returnvalue_2 (`self.GetAbilityLevel`))
  (if (`self.FirstTargetImplementsInterface`)
    (bind _output_get (set `local.ASC` _returnvalue))
    (bind _returnvalue_3 (`AbilitySystemBlueprintLibrary.AssignTagSetByCallerMagnitude` (`AbilitySystemComponent.MakeOutgoingSpec` _output_get (`self.DamageEffectClass`) (`KismetMathLibrary.Conv_IntToDouble` _returnvalue_2) (`AbilitySystemComponent.MakeEffectContext` _returnvalue)) (struct :`TagName` "Damage.Lightning") (`self.GetDamageAtLevel` _returnvalue_2)))
    (bind _output_get_2 (set `local.EffectContext` _returnvalue_3))
    (`AbilitySystemComponent.BP_ApplyGameplayEffectSpecToTarget` (`local.ASC`) _output_get_2 (`AbilitySystemBlueprintLibrary.GetAbilitySystemComponent` (`self.MouseHitActor`)))
    (bind _keypin (`|MapForEach` (`self.AdditionalTargetsToCueParams`))
      (:`then`
        (`AbilitySystemComponent.BP_ApplyGameplayEffectSpecToTarget` (`local.ASC`) (`local.EffectContext`) (`AbilitySystemBlueprintLibrary.GetAbilitySystemComponent` _keypin))))))

(fn `RemoveCueFromAddtionalTarget`
  (params (Target :type "Actor Object Reference"))
  (locals (TargetToRemoveCue :type "Actor Object Reference"))
  (bind _output_get (set `local.TargetToRemoveCue` Target))
  (bind (_value _returnvalue) (`BlueprintMapLibrary.Map_Find` (`self.AdditionalTargetsToCueParams`) _output_get))
  (if _returnvalue
    (`GameplayCueFunctionLibrary.RemoveGameplayCueOnActor` (`local.TargetToRemoveCue`) (struct :`TagName` "GameplayCue.Shock.Loop") _value)
    (`BlueprintMapLibrary.Map_Remove` (`self.AdditionalTargetsToCueParams`) (`local.TargetToRemoveCue`))))

(fn `RemoveCuesAndShock`
  (if (`self.FirstTargetImplementsInterface`)
    (bind (_keypin _valuepin) (`|MapForEach` (`self.AdditionalTargetsToCueParams`))
      (:`then`
        (`GameplayCueFunctionLibrary.RemoveGameplayCueOnActor` _keypin (struct :`TagName` "GameplayCue.Shock.Loop") _valuepin)
        (message `CombatInterface.SetInShockLoop` _keypin false))
      (:`CompletedPin`
        (`GameplayCueFunctionLibrary.RemoveGameplayCueOnActor` (`self.MouseHitActor`) (struct :`TagName` "GameplayCue.Shock.Loop") (`self.FirstTargetParams`))
        (message `CombatInterface.SetInShockLoop` (`self.MouseHitActor`) false)
        (`BlueprintMapLibrary.Map_Clear` (`self.AdditionalTargetsToCueParams`))))
    (else
      (`GameplayCueFunctionLibrary.RemoveGameplayCueOnActor` (`self.GetAvatarActorFromActorInfo`) (struct :`TagName` "GameplayCue.Shock.Loop") (`self.FirstTargetParams`)))))

(fn `SpawnBeam`
  (locals (CueTarget :type "Actor Object Reference"))
  (bind _returnvalue (`KismetSystemLibrary.DoesImplementInterface` (`self.MouseHitActor`) "/Script/Aura.CombatInterface"))
  (`self.TraceFirstTarget` (`self.MouseHitLocation`))
  (bind _returnvalue_2 (message `CombatInterface.GetWeaponMesh` (`self.GetAvatarActorFromActorInfo`)))
  (set `self.WeaponMesh` _returnvalue_2)
  (set `self.FirstTargetParams` (`AbilitySystemBlueprintLibrary.MakeGameplayCueParameters` 0.0 0.0 (struct) (struct) (struct) (struct) (struct) (`self.MouseHitLocation`) (0.0 0.0 0.0) null null (`self.MouseHitActor`) null 1 1 (`self.WeaponMesh`)))
  (set `self.FirstTargetImplementsInterface` _returnvalue)
  (if _returnvalue
    (bind _output_get (set `local.CueTarget` (`self.MouseHitActor`)))
    (message `CombatInterface.SetInShockLoop` _output_get true)
    (bind _outadditionaltargets (`self.StoreAdditionalTargets`))
    (for _array_element _outadditionaltargets
      (`self.AddCueToAdditionalTarget` _array_element)
      (message `CombatInterface.SetInShockLoop` _array_element true))
    (else
      (set `local.CueTarget` (`self.GetAvatarActorFromActorInfo`))))
  (`GameplayCueFunctionLibrary.AddGameplayCueOnActor` (`local.CueTarget`) (struct :`TagName` "GameplayCue.Shock.Loop") (`self.FirstTargetParams`)))