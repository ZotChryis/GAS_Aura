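; Arcane Shards gameplay ability that shows a magic circle for aiming, then erupts a series of damaging shards at the targeted ground.
; On confirm it commits cost and cooldown, then spawns a point collection at the cursor hit to generate randomly rotated ground points.
; A montage event starts a looping timer that fires a gameplay cue per point and applies radial knockback damage, ending after the last shard.
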(event `self.K2_ActivateAbility`
  ; Handle Aim->Cast Transition
  (message `PlayerInterface.ShowMagicCircle` (`self.GetAvatarActorFromActorInfo`))
  (`AbilityTask_WaitInputPress.WaitInputPress` false
    (:`OnPress`
      (message `PlayerInterface.HideMagicCircle` (`self.GetAvatarActorFromActorInfo`))
      ; Handle cooldown and cost
      (bind _returnvalue (`self.K2_CommitAbilityCost` false))
      (if _returnvalue
        (`self.K2_CommitAbilityCooldown` false)
        ; Handle targetting, generate points to spawn shards in
        (bind (_asynctaskproxy _datahandle) (`TargetDataUnderMouse.CreateTargetDataUnderMouse`)
          (:`Data`
            (bind (_bblockinghit _binitialoverlap _time _distance _location _impactpoint) (`GameplayStatics.BreakHitResult` (`AbilitySystemBlueprintLibrary.GetHitResultFromTargetData` _datahandle)))
            (message `CombatInterface.UpdateFacingTarget` (`self.GetAvatarActorFromActorInfo`) _impactpoint)
            (bind _returnvalue_2 (`|SpawnActorFromClass` "/Game/Blueprints/AbilitySystem/Aura/Ability/Arcane/ArcaneShards/BP_PointCollection.BP_PointCollection_C" (`KismetMathLibrary.MakeTransform` _impactpoint) "Undefined" "MultiplyWithRoot" null null))
            (set `self.PointCollectionActor` _returnvalue_2)
            (set `self.Points` (`PointCollection.GetGroundPoints` _returnvalue_2 _impactpoint (`self.NumPoints`) (`KismetMathLibrary.RandomFloatInRange` 0.0 360.0)))
            ; Animation
            (`AbilityTask_PlayMontageAndWait.CreatePlayMontageAndWaitProxy` "None" "/Game/Assets/Characters/Aura/Animations/Abilities/AM_Cast_ArcaneShards.AM_Cast_ArcaneShards"
              (:`then`
                (`AbilityTask_WaitGameplayEvent.WaitGameplayEvent` (struct :`TagName` "Event.Montage.ArcaneShards") null
                  (:`EventReceived`
                    ; Timer loop for number of shards
                    (bind _returnvalue_3 (`KismetSystemLibrary.K2_SetTimerDelegate` (delegate `SpawnShard`) (`self.ShardSpawnDeltaTime`) true))
                    (set `self.TimerHandle` _returnvalue_3)))))))
        (else
          (`self.K2_EndAbility`))))))

(event `SpawnShard`
  ; Spawn s shard
  (set `self.Origin` (`SceneComponent.K2_GetComponentLocation` (`|GetArrayItem` (`self.Points`) (`self.SpawnedShards`))))
  (`self.K2_ExecuteGameplayCueWithParams` (struct :`TagName` "GameplayCue.ArcaneShards") (`AbilitySystemBlueprintLibrary.MakeGameplayCueParameters` 0.0 0.0 (struct) (struct) (struct) (struct) (struct) (`self.Origin`)))
  ; Get stuff to damage in shard area
  (bind _outactors (`AuraAbilitySystemLibrary.GetLivePlayersWithinRadius` (`self.GetAvatarActorFromActorInfo`) (`|MakeArray` (`self.GetAvatarActorFromActorInfo`)) (`self.Origin`) (`self.RadialDamageOuterRadius`)))
  (for _array_element _outactors
    (bind _returnvalue (- (`Actor.K2_GetActorLocation` _array_element) (`self.Origin`)))
    ; Damage actor in area
    (`AuraAbilitySystemLibrary.ApplyDamageEffect` (`self.MakeDamageEffectParamsFromClassDefaults` _array_element (`self.Origin`) true _returnvalue true _returnvalue)))
  ; Check for spawned enough shards, exit
  (`/Engine/EditorBlueprintResources/StandardMacros.IncrementInt` (`self.SpawnedShards`)
    (:`  `
      (if (== (`self.SpawnedShards`) (`self.NumPoints`))
        (`KismetSystemLibrary.K2_ClearAndInvalidateTimerHandle` (`self.TimerHandle`))
        (`Actor.K2_DestroyActor` (`self.PointCollectionActor`))
        (`KismetSystemLibrary.Delay` 0.2)
        (`self.K2_EndAbility`)))))

(event `self.K2_OnEndAbility`
  (params (bWasCancelled :type Boolean)))