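; GA_Attack_Ranged is an enemy gameplay ability for a ranged attack that fires a projectile at the avatar's combat target.
; It turns the avatar toward the target through CombatInterface, then plays a random tagged attack montage.
; The montage's gameplay event triggers a single SpawnProjectile call, using the entry's socket tag, the target's current location and a pitch override.
; The ability ends when the montage completes, is interrupted or is cancelled.
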(event `self.K2_ActivateAbility`
  (bind _ascombat_interface (cast `CombatInterface` (`self.GetAvatarActorFromActorInfo`))
    (:`then`
      (set `self.CombatInterface` _ascombat_interface)
      (bind _returnvalue (message `EnemyInterface.GetCombatTarget` (`self.GetAvatarActorFromActorInfo`)))
      (`CombatInterface.UpdateFacingTarget` (`self.CombatInterface`) (`Actor.K2_GetActorLocation` _returnvalue))
      (bind _returnvalue_2 (`CombatInterface.GetAttackMontages` (`self.CombatInterface`)))
      (bind _output_get (set `self.TaggedMontage` (`KismetArrayLibrary.Array_Random` _returnvalue_2)))
      (bind (_montage _montagetag _sockettag) (break `TaggedMontage` _output_get))
      (`AbilityTask_PlayMontageAndWait.CreatePlayMontageAndWaitProxy` "None" _montage
        (:`then`
          (`AbilityTask_WaitGameplayEvent.WaitGameplayEvent` _montagetag null true
            (:`EventReceived`
              (`CombatInterface.GetCombatSocketLocation` (`self.CombatInterface`) _montagetag)
              (bind _returnvalue_3 (message `EnemyInterface.GetCombatTarget` (`KismetSystemLibrary.Conv_InterfaceToObject` (`self.CombatInterface`))))
              (`self.SpawnProjectile` (`Actor.K2_GetActorLocation` _returnvalue_3) _sockettag (`self.Pitch Override`)))))
        (:`OnCompleted`
          (`self.K2_EndAbility` :!label _label))
        (:`OnInterrupted`
          (goto _label))
        (:`OnCancelled`
          (goto _label))))
    (:`CastFailed`
      (`self.K2_EndAbility`))))