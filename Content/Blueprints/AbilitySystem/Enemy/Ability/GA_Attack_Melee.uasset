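; GA_Attack_Melee is an enemy melee attack gameplay ability that damages nearby opposing players during a montage.
; On activation it faces the combat target, plays a random tagged attack montage and waits for that montage's gameplay event.
; On the event it damages hostile live players in a small radius around the montage's combat socket, firing a melee impact GameplayCue on any hit.
; The ability ends when the montage completes or is interrupted or cancelled.
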(event `self.K2_ActivateAbility`
  (bind _returnvalue (`self.GetAvatarActorFromActorInfo`))
  (bind _returnvalue_2 (`self.GetAvatarActorFromActorInfo`))
  (set `self.HasHitTarget` false)
  (bind _ascombat_interface (cast `CombatInterface` (`self.GetAvatarActorFromActorInfo`))
    (:`then`
      (set `self.CombatInterface` _ascombat_interface)
      (bind _returnvalue_3 (message `EnemyInterface.GetCombatTarget` (`self.GetAvatarActorFromActorInfo`)))
      (`CombatInterface.UpdateFacingTarget` _ascombat_interface (`Actor.K2_GetActorLocation` _returnvalue_3))
      (bind _returnvalue_4 (message `CombatInterface.GetAttackMontages` (`self.GetAvatarActorFromActorInfo`)))
      (bind _output_get (set `self.TaggedMontage` (`KismetArrayLibrary.Array_Random` _returnvalue_4)))
      (bind (_montage _montagetag _sockettag) (break `TaggedMontage` _output_get))
      (`AbilityTask_PlayMontageAndWait.CreatePlayMontageAndWaitProxy` "None" _montage
        (:`then`
          (`AbilityTask_WaitGameplayEvent.WaitGameplayEvent` _montagetag null
            (:`EventReceived`
              (bind _returnvalue_5 (`CombatInterface.GetCombatSocketLocation` (`self.CombatInterface`) _sockettag))
              (set `self.CombatSocketLocation` _returnvalue_5)
              (bind _outactors (`AuraAbilitySystemLibrary.GetLivePlayersWithinRadius` _returnvalue_2 (`|MakeArray` _returnvalue_2) (`self.CombatSocketLocation`) 50.0))
              (for _array_element _outactors
                (if (`AuraAbilitySystemLibrary.AreEnemies` _array_element (`self.GetAvatarActorFromActorInfo`))
                  (set `self.HasHitTarget` true)
                  (`AuraAbilitySystemLibrary.ApplyDamageEffect` (`self.MakeDamageEffectParamsFromClassDefaults` _array_element))))
              (if (`self.HasHitTarget`)
                (bind _returnvalue_6 (message `EnemyInterface.GetCombatTarget` _returnvalue))
                (`self.K2_ExecuteGameplayCueWithParams` (struct :`TagName` "GameplayCue.MeleeImpact") (`AbilitySystemBlueprintLibrary.MakeGameplayCueParameters` 0.0 0.0 (struct) (struct) (struct) (`BlueprintGameplayTagLibrary.MakeGameplayTagContainerFromTag` (`.MontageTag` (break `TaggedMontage` (`self.TaggedMontage`)))) (struct) (`self.CombatSocketLocation`) (0.0 0.0 0.0) null _returnvalue _returnvalue_6))))))
        (:`OnCompleted`
          (`self.K2_EndAbility` :!label _label))
        (:`OnInterrupted`
          (goto _label))
        (:`OnCancelled`
          (goto _label))))
    (:`CastFailed`
      (`self.K2_EndAbility`))))