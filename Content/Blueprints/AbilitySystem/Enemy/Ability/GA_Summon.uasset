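; GA_Summon is an enemy gameplay ability for summoning that currently only previews spawn points with debug spheres.
; On activation it stores the results of GetSpawnLocations and shuffles them.
; A delayed loop then steps an index through the array, briefly drawing one sphere at each location in turn.
; The graph spawns no actors and never calls EndAbility.
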(event `self.K2_ActivateAbility`
  (bind _returnvalue (`self.GetSpawnLocations`))
  (bind _output_get (set `self.SpawnLocations` _returnvalue))
  (`KismetArrayLibrary.Array_Shuffle` _output_get)
  (if (< (`self.SpawnLocationIndex`) (`KismetArrayLibrary.Array_Length` (`self.SpawnLocations`))) :!label _label
    (`KismetSystemLibrary.DrawDebugSphere` (`|GetArrayItem` (`self.SpawnLocations`) (`self.SpawnLocationIndex`)) 10.0 12 (struct :`R` 1.0 :`G` 0.041667 :`B` 0.816052 :`A` 1.0) 1.0 1.0)
    (set `self.SpawnLocationIndex` (+ (`self.SpawnLocationIndex`) 1))
    (`KismetSystemLibrary.Delay` 0.2)
    (goto _label)))