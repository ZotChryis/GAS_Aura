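; Main menu scene actor that plays menu music, shows the WBP_MainMenu widget and animates a fireball and a magic circle decal.
; BeginPlay stores the fireball's start location, sets UI-only input focused on the widget and shows the mouse cursor.
; Tick bobs the fireball vertically on a sine of an accumulated time that resets after a full period, and spins the decal at a configurable rate.
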(event `self.ReceiveBeginPlay`
  (bind _returnvalue (`GameplayStatics.GetPlayerController` 0))
  (set `self.FireballInitialLocation` (`SceneComponent.K2_GetComponentLocation` (`self.Fireball`)))
  (`GameplayStatics.PlaySound2D` "/Game/Assets/Sounds/Music/Music_MainMenu.Music_MainMenu" 1.0 1.0 0.0 null null)
  (bind _returnvalue_2 (`|CreateWidget` "/Game/Blueprints/MainMenu/WBP_MainMenu.WBP_MainMenu_C"))
  (`UserWidget.AddToViewport` _returnvalue_2 0)
  (`WidgetBlueprintLibrary.SetInputMode_UIOnlyEx` _returnvalue _returnvalue_2)
  (set `PlayerController.bShowMouseCursor` true _returnvalue))

(event `self.ReceiveTick`
  (params (DeltaSeconds :type "Float (single-precision)"))
  (`self.UpdateTime` DeltaSeconds)
  (`SceneComponent.K2_SetWorldLocation` (`self.Fireball`) (+ (`self.FireballInitialLocation`) (`KismetMathLibrary.MakeVector` 0.0 0.0 (`self.SinTime`))) false false)
  (`SceneComponent.K2_AddLocalRotation` (`self.Decal`) (`KismetMathLibrary.MakeRotator` (* (`GameplayStatics.GetWorldDeltaSeconds`) (`self.MagicCircleRotRate`))) false false))

(fn `SinTime`
  (returns (ReturnValue :type "Float (double-precision)"))
  (return (* (`KismetMathLibrary.Sin` (`self.Time`)) (`self.Amplitude`))))

(fn `UpdateTime`
  (params (DeltaTime :type "Float (double-precision)"))
  (bind _output_get (set `self.Time` (+ DeltaTime (`self.Time`))))
  (if (>= _output_get (* (`KismetMathLibrary.GetPI`) 2.0))
    (set `self.Time` 0.0)))

(fn `UserConstructionScript`)